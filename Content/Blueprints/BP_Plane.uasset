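; BP_Plane is a plane actor built to fly along a spline with a spinning propeller, though neither behavior is currently triggered.
; The Vol timeline, rate-scaled by Duration, samples the spline at constant velocity to place Scene1, offsetting yaw by -90 degrees.
; A second timeline lerps Scene's pitch toward a full turn for the propeller.
; BeginPlay and the construction script are empty, leaving both timeline chains disconnected.
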(event `self.ReceiveBeginPlay`
  ;[1 1 1] Vol
)

(fn `UserConstructionScript`)