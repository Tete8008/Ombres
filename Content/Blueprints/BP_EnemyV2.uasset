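; Patrolling enemy AI that chases the player character on sight and ends the game on catching them.
; It wanders between random navigable points, switching to run speed and a target-following AIMoveTo when PawnSensing spots the character.
; Tick counts down a lose-sight timer, after which a confusion timeline leads into walking back to spawn and patrolling again.
; Reaching or hitting the player shows the game-over overlay and disables input, unless they are using a spell.
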(event `self.ReceiveBeginPlay`
  ;[1 1 1] Init
  (set `self.StartingPosition` (`self.K2_GetActorLocation`))
  (set `self.InitialMaterial` (`PrimitiveComponent.GetMaterial` (`self.Mesh`) 2))
  (if (`self.CanMove`)
    (`self.Routine`)))

(event `self.PawnSensing.OnSeePawn`
  (params (Pawn :type "Pawn Object Reference"))
  (bind (_asbp_character _bsuccess) (cast `/Game/Blueprints/BP_Character` Pawn :!pure true))
  ;[1 1 1] Character detection
  (if (and _bsuccess (`self.CanMove`))
    (set `self.TimeLeftBeforeLosingCharacter` (`self.TimeBeforeLosingCharacter`))
    ;[1 1 1] Chase Character
    (if (not (`self.Chasing`))
      (set `self.TargetedPlayer` _asbp_character)
      (set `self.Chasing` true)
      (set `CharacterMovementComponent.MaxWalkSpeed` (`self.RunSpeed`) (`self.CharacterMovement`))
      (`NavMovementComponent.StopActiveMovement` (`self.CharacterMovement`))
      (`|AIMoveTo` self (0.0 0.0 0.0) (`self.TargetedPlayer`) 10.0 :!label _label
        (:`then`
          ;[1 1 1] Character lost -> enemy confused
          (`Timeline|OMGIMLOST` :!via `Stop` :!label _label_2 ; Wait a few seconds
            (:`Finished`
              ;[1 1 1] Return to initial position
              (set `CharacterMovementComponent.MaxWalkSpeed` (`self.WalkSpeed`) (`self.CharacterMovement`))
              (`|AIMoveTo` self (`self.StartingPosition`) null
                (:`OnSuccess`
                  _)
                (:`OnFail`
                  _))
              (`self.Routine`))))
        (:`OnSuccess`
          (if (not (`/Game/Blueprints/BP_Character.IsUsingSpell` (`self.TargetedPlayer`)))
            (`self.CatchPlayer`)))
        (:`OnFail`
          (if (> (`self.TimeLeftBeforeLosingCharacter`) 0.0)
            (goto _label)
            (else
              (set `self.Chasing` false :!label _label_3)
              (`NavMovementComponent.StopActiveMovement` (`self.CharacterMovement`))
              (`TimelineComponent.SetPlayRate` (`self.OMGIMLOST`) (/ 1.0 (`self.ConfusedDuration`)))
              (goto _label_2 :!via `PlayFromStart`))))))))

(event `Routine`
  ;[1 1 1] Enemy routine
  (`|AIMoveTo` self (`NavigationSystemV1.K2_GetRandomLocationInNavigableRadius` (`self.K2_GetActorLocation`) 10000.0 null null) null
    (:`OnSuccess`
      _)
    (:`OnFail`
      _))
  (`KismetSystemLibrary.Delay` 3.0)
  (if (not (`self.Chasing`))
    (`self.Routine`)))

(event `self.ReceiveTick`
  (params (DeltaSeconds :type "Float (single-precision)"))
  ;[1 1 1] Time before losing character
  (if (`self.Chasing`)
    (bind _output_get (set `self.TimeLeftBeforeLosingCharacter` (- (`self.TimeLeftBeforeLosingCharacter`) DeltaSeconds)))
    (if (<= _output_get 0.0)
      (goto _label_3))))

(event `CatchPlayer`
  (bind _returnvalue (`GameplayStatics.GetPlayerController` 0))
  ;[1 1 1] Catch player
  (bind _returnvalue_2 (`|CreateWidget` "/Game/UI/GameOverOverlay.GameOverOverlay_C"))
  (`UserWidget.AddToViewport` _returnvalue_2 0)
  (set `PlayerController.bShowMouseCursor` true _returnvalue)
  (`self.DisableInput` (`GameplayStatics.GetPlayerPawn` 0) _returnvalue))

(event `self.ReceiveHit`
  (params (MyComp :type "PrimitiveComponent Object Reference") (Other :type "Actor Object Reference") (OtherComp :type "PrimitiveComponent Object Reference") (bSelfMoved :type Boolean) (HitLocation :type "Vector Structure") (HitNormal :type "Vector Structure") (NormalImpulse :type "Vector Structure") (Hit :type "HitResult Structure (by ref)"))
  (bind (_asbp_character _bsuccess) (cast `/Game/Blueprints/BP_Character` Other :!pure true))
  (if _bsuccess
    (if (not (`/Game/Blueprints/BP_Character.IsUsingSpell` _asbp_character))
      (`self.CatchPlayer`))))

(fn `UserConstructionScript`)