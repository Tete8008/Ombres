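; BP_Platform is a platform actor that destroys itself if a BP_Character hits it while its JustSpawned flag is set.
; While Zbeub is true, Tick steps through boolean flags: it sets Starting, then raises JustSpawned, then clears both JustSpawned and Zbeub on successive frames.
; This frame-counted latch limits self-destruction to a brief window, apparently rejecting platforms that spawn touching the character.
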(event `self.ReceiveTick`
  (params (DeltaSeconds :type "Float (single-precision)"))
  (if (`self.Zbeub`)
    (if (`self.Starting`)
      (if (`self.JustSpawned`)
        (set `self.JustSpawned` false)
        (set `self.Zbeub` false)
        (else
          (set `self.JustSpawned` true)))
      (else
        (set `self.Starting` true)))))

(event `self.ReceiveHit`
  (params (MyComp :type "PrimitiveComponent Object Reference") (Other :type "Actor Object Reference") (OtherComp :type "PrimitiveComponent Object Reference") (bSelfMoved :type Boolean) (HitLocation :type "Vector Structure") (HitNormal :type "Vector Structure") (NormalImpulse :type "Vector Structure") (Hit :type "HitResult Structure (by ref)"))
  (if (`.bSuccess` (cast `/Game/Blueprints/BP_Character` Other :!pure true))
    (if (`self.JustSpawned`)
      (`self.K2_DestroyActor`))))

(fn `UserConstructionScript`)